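; BP_Spark is a casting effect actor that emits a repeating spark beam along its forward direction until something overlaps it.
; On BeginPlay it spawns the NS_Spark Niagara system, then respawns it on a fast looping timer at the actor's current location and facing, with a stretched scale.
; Any actor overlap destroys it.
; A BeamEnd vector parameter setter is left unwired, and Tick is unused.
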(event Custom|SpawnBeam
  (Niagara|SpawnSystematLocation "/Game/VFX/NS_Spark.NS_Spark" (Transformation|GetActorLocation) (Math|Conversions|RotationFromXVector (Math|Vector|GetForwardVector (Transformation|GetActorRotation))) "5.000000,2.000000,2.000000"))

(event EventBeginPlay
  (CallFunction|SpawnBeam)
  (Utilities|Time|SetTimerbyEvent (delegate Custom|SpawnBeam) 0.075 true))

(event Collision|EventActorBeginOverlap
  (params (OtherActor :type Actor%20Object%20Reference))
  (Actor|DestroyActor))

(event EventTick
  (params (DeltaSeconds :type Float%20%28single-precision%29)))

(fn ConstructionScript)