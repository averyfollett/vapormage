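; First-person player character Blueprint that handles blocking, cast animation and right-stick UI feedback.
; Each tick it spawns a BP_Block at the camera transform while either block side is active, feeds stick input to the WB_PlayerUI widget component, and plays the cast montage on the first-person mesh while casting.
; Hotkeys apply test damage with camera shake, restart the level or open the main menu.
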(event Custom|Blocking
  (bind _playerstatus (Variables|Default|GetPlayerStatus))
  (if (or (.bisblockingleft _playerstatus) (.bisblockingright _playerstatus))
    (Game|SpawnActorfromClass "/Game/Blueprints/Casting/BP_Block.BP_Block_C" (Transformation|GetWorldTransform (Variables|Default|GetFirstPersonCameraComponent)) "Undefined" 0 0)))

(event EventTick
  (params (DeltaSeconds :type Float%20%28single-precision%29))
  (CallFunction|Blocking)
  ;[1 1 1] Sends RStick position to PlayerUI to update the widget's position.
  (bind _aswb_player_ui (Utilities|Casting|CastToWB_PlayerUI (UserInterface|GetUserWidgetObject (Variables|Default|GetPlayerUI))))
  (Default|UpdateRStickPosition _aswb_player_ui (Class|Actor|GetInputAxisKeyValue) (Class|Actor|GetInputAxisKeyValue))
  (if (Variables|Default|GetbAnimIsCasting)
    (Animation|Montage|MontagePlay (Components|SkeletalMesh|GetAnimInstance (Variables|Default|GetMesh1P)) "/Game/Animations/AM_Cast.AM_Cast" 1.0 "MontageLength" 0.0 true)))

(event Input|KeyboardEvents|7
  (params (Key :type Key%20Structure :default "None"))
  (:Pressed
    (Class|PlayerCharacter|DamagePlayer 1e+01 false)
    (Class|PlayerController|ClientPlayCameraShake (Game|GetPlayerController 0) "/Game/Blueprints/CameraShake/BP_DamageTakenShake.BP_DamageTakenShake_C" 1.0 "CameraLocal" "0, 0, 0")))

(event Input|KeyboardEvents|R
  (params (Key :type Key%20Structure :default "None"))
  ;[1 1 1] Reset level or return to MainMenu.
  (:Pressed
    (bind _returnvalue (Game|GetCurrentLevelName true))
    (Game|OpenLevel(byName) (Utilities|String|StringToName _returnvalue))))

(event Input|GamepadEvents|GamepadSpecialRight
  (params (Key :type Key%20Structure :default "None"))
  ;[1 1 1] Reset level or return to MainMenu.
  (:Pressed
    (Game|OpenLevel(byName) "LV_MainMenu")))

(fn ConstructionScript)